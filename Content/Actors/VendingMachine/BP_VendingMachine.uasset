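; BP_VendingMachine is an interactable vending machine that gives the player a weapon after a timed hold interaction.
; A WBP_Interaction widget, created on BeginPlay, shows or hides as interaction is enabled or disabled.
; While interacting, Tick fills a progress value over SecondsToInteract, exposed through GetInteractValue and reset when interaction stops.
; On completion it disables itself and calls SpawnWeapon on the player's WeaponManager with its GunSetting.
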(event EventEnableInteraction
  (Development|SetHiddeninGame (Variables|Default|GetWidget) false false)
  (Variables|Default|SetCanInteract true))

(event EventDisableInteraction
  (Development|SetHiddeninGame (Variables|Default|GetWidget) true false)
  (Variables|Default|SetCanInteract false))

(event EventStartInteract
  (Variables|Default|SetInteracting true))

(event EventStopInteract
  (Variables|Default|SetInteracting false))

(event EventTick
  (params (DeltaSeconds :type Float%20%28single-precision%29))
  (if (and (Variables|Default|GetInteracting) (Variables|Default|GetCanInteract))
    (if (< (Variables|Default|GetValue) 1.0)
      (bind _output_get (Variables|Default|SetValue (+ (/ DeltaSeconds (Variables|Default|GetSeconds%20to%20Interact)) (Variables|Default|GetValue))))
      (if (>= _output_get 1.0)
        (Variables|Default|SetCanInteract false)
        (Development|SetHiddeninGame (Variables|Default|GetWidget) true false)
        (Default|SpawnWeapon (Actor|GetComponentbyClass (Game|Player|GetPlayerPawn 0) "/FPSAnimationPack/Blueprints/Character/WeaponManager.WeaponManager_C") (Variables|Default|GetGunSetting))))
    (else
      (Variables|Default|SetValue 0.0))))

(event EventBeginPlay
  (bind _returnvalue (UserInterface|CreateWidget "/Game/UI/WBP_Interaction.WBP_Interaction_C" 0 self))
  (UserInterface|SetWidget (Variables|Default|GetWidget) _returnvalue))

(fn ConstructionScript)

(fn GetInteractValue
  (return (Variables|Default|GetValue)))
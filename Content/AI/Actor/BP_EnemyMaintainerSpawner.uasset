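; BP_EnemyMaintainerSpawner manages which enemy types are in play by spawning a BP_EnemyMaintainer for each.
; On BeginPlay it starts a set number of maintainers, passing each a random enemy type, the spawn points, a spawn limit and a self reference.
; Each chosen type leaves the available pool, so none repeats.
; It binds to each maintainer's SpawnNewType event, apparently to bring in replacement types until the pool empties.
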(event EventBeginPlay
  (for _index (range 0 (- (Variables|Default|GetNoOfEnemyTypesAtOnce) 1))
    (CallFunction|SpawnNewType)))

(fn ConstructionScript)

(fn SpawnNewType
  (bind (_outitem _outindex) (Utilities|Array|Random (Variables|Default|GetAvailableEnemyTypes)))
  (if (>= _outindex 0)
    (bind _returnvalue (Game|SpawnActorfromClass "/Game/AI/Actor/BP_EnemyMaintainer.BP_EnemyMaintainer_C" (Math|Transform|MakeTransform "0, 0, 0" "0, 0, 0" "1.000000,1.000000,1.000000") "Undefined" "MultiplyWithRoot" 0 (Variables|Default|GetSpawnPoints) _outitem (Variables|Default|GetNoOfTimestoSpawnOneEnemy) self 0))
    (EventDispatchers|BindEventtoSpawnNewType _returnvalue (EventDispatchers|CreateEvent :!event SpawnNewType))
    (Utilities|Array|RemoveIndex (Variables|Default|GetAvailableEnemyTypes) _outindex)))
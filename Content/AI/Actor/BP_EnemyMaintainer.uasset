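; BP_EnemyMaintainer spawns enemies of one type, set by a data asset, up to a maximum total.
; BeginPlay spawns one BP_EnemyBase at a random reachable point near a random spawning location offset from the spawner reference.
; Each spawn increments a counter and binds an event to the enemy's OnDead.
; Once the cap is reached, a further spawn call fires the SpawnNewType dispatcher instead.
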(event EventBeginPlay
  (CallFunction|SpawnEnemy))

(fn ConstructionScript)

(fn SpawnEnemy
  (if (< (Variables|Default|GetEnemiesSpawned) (Variables|Default|GetMaxNumberToSpawn))
    (bind _returnvalue (Game|SpawnActorfromClass "/Game/AI/BP/BP_EnemyBase.BP_EnemyBase_C" (Math|Transform|MakeTransform (.RandomLocation (AI|Navigation|GetRandomReachablePointinRadius (+ (.OutItem (Utilities|Array|Random (Variables|Default|GetSpawningLocations))) (Transformation|GetActorLocation (Variables|Default|GetSpawerRef))) 5e+02 0 0)) "0, 0, 0" "1.000000,1.000000,1.000000") "AdjustIfPossibleButAlwaysSpawn" "MultiplyWithRoot" 0 (Variables|Default|GetEnemyType) 0))
    (Math|Integer|IncrementInt (Variables|Default|GetEnemiesSpawned)
      (:%20%20
        (EventDispatchers|BindEventtoOnDead _returnvalue (EventDispatchers|CreateEvent :!event SpawnEnemy))))
    (else
      (Default|CallSpawnNewType))))
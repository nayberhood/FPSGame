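; Base enemy that chases player 0 at a random walk or run speed and attacks within range.
; Tick switches between AI MoveTo and timed forward sphere-trace attacks that apply damage.
; Incoming hits spawn blood and deal heavy damage high on the body, triggering a one-time low-health stagger, then death.
; A data asset supplies mesh, animations and capsule sizes, played directly on the mesh without an AnimBP state machine.
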(event Custom|Walk/Run%20Towards%20Player
  (bind _dataasset (Variables|Default|GetDataAsset))
  (Variables|Default|SetAttackStarted false)
  (Variables|Default|SetWalkStarted true)
  (Variables|/Script/Engine.CharacterMovementComponent|SetMaxWalkSpeed (Variables|Character|GetCharacterMovement) (Math|Random|RandomFloatinRange 2.5e+02 4.5e+02))
  (Components|Animation|PlayAnimation (Variables|Character|GetMesh) (select (Math|Float|InRange(Float) (Variables|/Script/Engine.CharacterMovementComponent|GetMaxWalkSpeed (Variables|Character|GetCharacterMovement)) 2.5e+02 325.0) (Variables|/Game/AI/Data/EnemyDataAssetClass.EnemyDataAssetClass_C|GetWalkAnim _dataasset) (Variables|/Game/AI/Data/EnemyDataAssetClass.EnemyDataAssetClass_C|GetRunAnim _dataasset)) true)
  (AI|AIMoveTo self "0, 0, 0" (Game|Player|GetPlayerPawn 0) 1.5e+02 false
    (:OnSuccess
      _)
    (:OnFail
      _))
  (Variables|Default|SetWalkStarted false))

(event Custom|Attack
  (bind _returnvalue (Transformation|GetActorLocation))
  (Variables|Default|SetAttackStarted true)
  (Components|Animation|PlayAnimation (Variables|Character|GetMesh) (Variables|/Game/AI/Data/EnemyDataAssetClass.EnemyDataAssetClass_C|GetAttackAnim (Variables|Default|GetDataAsset)) true)
  (bind _outhit (Class|KismetSystemLibrary|SphereTraceSinglebyProfile _returnvalue (+ _returnvalue (* (Transformation|GetActorForwardVector) 2.5e+02)) 75.0 "Pawn" false 0 "None" true))
  (Game|Damage|ApplyDamage (.hitactor _outhit) (Variables|Default|GetBase%20Damage) 0 0)
  (Utilities|FlowControl|Delay (Variables|Default|GetDurationBetweenAttacks))
  (Variables|Default|SetAttackStarted false))

(event Custom|GetHit
  (bind _dataasset (Variables|Default|GetDataAsset))
  (bind _gethitanim (Variables|/Game/AI/Data/EnemyDataAssetClass.EnemyDataAssetClass_C|GetGetHitAnim _dataasset))
  (if (not (Variables|Default|GetGetHitPlayed))
    (Variables|Default|SetPlayingHit true)
    (Variables|Default|SetGetHitPlayed true)
    (AI|Navigation|StopMovement (AI|GetAIController self))
    (Components|Animation|PlayAnimation (Variables|Character|GetMesh) _gethitanim false)
    (Utilities|FlowControl|Delay (Animation|GetPlayLength _gethitanim))
    (Variables|Default|SetPlayingHit false)))

(event Custom|Die
  (bind _capsulecomponent (Variables|Collision|GetCapsuleComponent))
  (Variables|Default|SetDead true)
  (Components|Animation|PlayAnimation (Variables|Character|GetMesh) (Variables|/Game/AI/Data/EnemyDataAssetClass.EnemyDataAssetClass_C|GetDeathAnim (Variables|Default|GetDataAsset)) false)
  (Collision|SetCollisionObjectType _capsulecomponent "ECC_Visibility")
  (Collision|SetCollisionResponsetoAllChannels _capsulecomponent "ECR_Ignore")
  (Collision|SetCollisionResponsetoChannel (Variables|Collision|GetCapsuleComponent) "ECC_WorldStatic" "ECR_Block")
  (AI|Navigation|StopMovement (AI|GetAIController self)))

(event EventTick
  (params (DeltaSeconds :type Float%20%28single-precision%29))
  (if (not (Variables|Default|GetDead))
    (if (Math|Float|InRange(Float) (Math|Vector|Distance2D(Vector) (Transformation|GetActorLocation) (Transformation|GetActorLocation (Game|Player|GetPlayerPawn 0))) 0.0 2.5e+02)
      (if (not (Variables|Default|GetAttackStarted))
        (CallFunction|Attack))
      (elif (not (Variables|Default|GetPlayingHit))
        (if (not (Variables|Default|GetWalkStarted))
          (CallFunction|Walk/RunTowardsPlayer))))))

(event EventApplyDamage
  (params (Hit%20Result :type Hit%20Result%20Structure))
  (bind _location (Collision|BreakHitResult Hit%20Result))
  (Niagara|SpawnSystematLocation "/Game/RealisticBlood/Burst/Niagara/NS_BloodBurst_Low.NS_BloodBurst_Low" _location)
  (if (not (Variables|Default|GetDead))
    (bind _output_get (Variables|Default|SetHealth (- (Variables|Default|GetHealth) (Math|Float|SelectFloat 1e+02 1e+01 (< (- (.z (Transformation|GetActorLocation)) (.Z (Math|Vector|BreakVector _location))) -3e+01)))))
    (if (<= _output_get 25.0)
      (CallFunction|GetHit)
      (if (<= (Variables|Default|GetHealth) 0.0)
        (CallFunction|Die)))))

(event EventBeginPlay
  (AI|SetFocus (AI|GetAIController self) (Game|Player|GetPlayerPawn 0))
  (CallFunction|Walk/RunTowardsPlayer))

(fn ConstructionScript
  (Components|SkeletalMesh|SetSkeletalMeshAsset (Variables|Character|GetMesh) (Variables|/Game/AI/Data/EnemyDataAssetClass.EnemyDataAssetClass_C|GetCharacterMesh (Variables|Default|GetDataAsset)))
  (Components|Capsule|SetCapsuleRadius (Variables|Collision|GetCapsuleComponent) (Variables|/Game/AI/Data/EnemyDataAssetClass.EnemyDataAssetClass_C|GetCapsuleRadius (Variables|Default|GetDataAsset)) true)
  (Components|Capsule|SetCapsuleHalfHeight (Variables|Collision|GetCapsuleComponent) (Variables|/Game/AI/Data/EnemyDataAssetClass.EnemyDataAssetClass_C|GetCapsuleHeight (Variables|Default|GetDataAsset)) true)
  (Transformation|AttachComponentToComponent (Variables|Default|GetCapsule) (Variables|Character|GetMesh) "Hips" "KeepRelative" "KeepRelative" "KeepRelative" true))
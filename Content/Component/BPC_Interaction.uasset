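; BPC_Interaction is an interaction component that detects interactable objects under the player's view and relays interact input to them.
; Each tick it line-traces from the camera for BPI_Interactable actors, caching one and toggling its interaction message and the IMC_Interact mapping context.
; IA_Interact sends start and stop interface messages to the cached object.
; The cached object changes only after the trace leaves all interactables.
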(event Input|EnhancedActionEvents|EnhancedInputActionIA_Interact
  (params (ActionValue :type Boolean) (ElapsedSeconds :type Float%20%28double-precision%29) (TriggeredSeconds :type Float%20%28double-precision%29) (InputAction :type Input%20Action%20Object%20Reference :default "/Game/Interactable/Input/Action/IA_Interact.IA_Interact"))
  (bind _interactionobject (Variables|Default|GetInteractionObject))
  (:Started
    (Class|BPIInteractable|StartInteract(Message) _interactionobject))
  (:Canceled
    (Class|BPIInteractable|StopInteract(Message) _interactionobject :!label _label))
  (:Completed
    (goto _label)))

(event EventTick
  (params (DeltaSeconds :type Float%20%28single-precision%29))
  (bind _returnvalue (Game|GetPlayerCameraManager 0))
  (bind _returnvalue_2 (Game|GetPlayerController 0))
  (bind _returnvalue_3 (Transformation|GetActorLocation _returnvalue))
  (bind _returnvalue_4 (PlayerController|LocalPlayerSubsystems|GetEnhancedInputLocalPlayerSubsystem _returnvalue_2))
  (bind _outhit (Collision|LineTraceByChannel _returnvalue_3 (+ _returnvalue_3 (* (Transformation|GetActorForwardVector _returnvalue) (Variables|Default|GetInteractionCheckDistance))) "TraceTypeQuery1" false (Utilities|Array|MakeArray (Game|Player|GetPlayerPawn 0)) "None"))
  (if (Utilities|DoesObjectImplementInterface (.hitactor _outhit) "/Game/Interactable/BPI_Interactable.BPI_Interactable_C")
    (Variables|Default|GetInteractionObject
      (:then)
      (:else
        (bind _output_get (Variables|Default|SetInteractionObject (.hitactor _outhit)))
        (Class|BPIInteractable|EnableInteraction(Message) _output_get)
        (Input|AddMappingContext _returnvalue_4 "/Game/Interactable/Input/IMC_Interact.IMC_Interact" 1 "(bIgnoreAllPressedKeysUntilRelease=True,bForceImmediately=False,bNotifyUserSettings=False)")))
    (else
      (bind _interactionobject (Variables|Default|GetInteractionObject)
        (:then
          (Class|BPIInteractable|DisableInteraction(Message) _interactionobject)
          (Variables|Default|SetInteractionObject 0)
          (Input|RemoveMappingContext _returnvalue_4 "/Game/Interactable/Input/IMC_Interact.IMC_Interact" "(bIgnoreAllPressedKeysUntilRelease=True,bForceImmediately=False,bNotifyUserSettings=False)"))
        (:else)))))